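; Trigger actor that spawns a ring of enemies when something begins overlapping its Box.
; On overlap it loops up to Quantity, spacing Enemy spawns at equal yaw steps at Radius around the actor's location.
; It then destroys itself, so it fires only once, with no filter on the overlapping actor.
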(event `self.Box.OnComponentBeginOverlap`
  (params (OverlappedComponent :type "PrimitiveComponent Object Reference") (OtherActor :type "Actor Object Reference") (OtherComp :type "PrimitiveComponent Object Reference") (OtherBodyIndex :type Integer) (bFromSweep :type Boolean) (SweepResult :type "HitResult Structure (by ref)"))
  (bind _quantity (`self.Quantity`))
  (set `self.CenterOfCircle` (`self.K2_GetActorLocation`))
  (for _index (range 1 (+ _quantity 1))
    (`|SpawnActorFromClass` "/Game/Blueprints/Enemy.Enemy_C" (`KismetMathLibrary.MakeTransform` (+ (* (`KismetMathLibrary.GetForwardVector` (`KismetMathLibrary.MakeRotator` 0.0 0.0 (`KismetMathLibrary.Conv_IntToDouble` (* _index (/ 360 _quantity))))) (`self.Radius`)) (`self.CenterOfCircle`))) "Undefined" "OverrideRootScale" null null))
  (`self.K2_DestroyActor`))

(fn `UserConstructionScript`)