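; Attacker drone that periodically stuns a random Enemy actor in the level and prints a debug message.
; Tick uses a Delay as its attack timer, then picks from all Enemy actors.
; BeginPlay caches four marker positions as patrol points before scattering the markers randomly in X/Y, then picks a point.
; The timeline that would lerp the drone between points is never run, so patrol movement is inactive.
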(event `self.ReceiveBeginPlay`
  (bind _asplayer (cast `/Game/Blueprints/Player` (`GameplayStatics.GetPlayerCharacter` 0)))
  (set `self.Player` _asplayer)
  (set `self.PatrolPoints` (`|MakeArray` (`SceneComponent.K2_GetComponentLocation` (`self.MovePosition1`)) (`SceneComponent.K2_GetComponentLocation` (`self.MovePosition2`)) (`SceneComponent.K2_GetComponentLocation` (`self.MovePosition3`)) (`SceneComponent.K2_GetComponentLocation` (`self.MovePosition4`))))
  (`self.SetRandomMovePosition`)
  (`self.GetRandomLocation`))

(event `self.ReceiveTick`
  (params (DeltaSeconds :type "Float (single-precision)"))
  (`KismetSystemLibrary.Delay` (`self.TimeBetweenAttacking`))
  (bind _outactors (`GameplayStatics.GetAllActorsOfClass` "/Game/Blueprints/Enemy.Enemy_C"))
  (if (`KismetArrayLibrary.Array_IsValidIndex` _outactors)
    (`/Game/Blueprints/Enemy.Stunned` (`|GetArrayItem` _outactors (`KismetMathLibrary.RandomIntegerInRange` 0 (- (`KismetArrayLibrary.Array_Length` _outactors) 1))))
    (`KismetSystemLibrary.PrintString` "Stunned Enemy")))

(fn `GetRandomLocation`
  (set `self.CurrentPatrolPoint` (`KismetMathLibrary.RandomIntegerInRange` 0 (- (`KismetArrayLibrary.Array_Length` (`self.PatrolPoints`)) 1))))

(fn `SetRandomMovePosition`
  (bind (_returnvalue_x _returnvalue_y _returnvalue_z) (`KismetMathLibrary.BreakVector` (`self.K2_GetActorLocation`)))
  (bind (_returnvalue_x_2 _returnvalue_y_2 _returnvalue_z_2) (`KismetMathLibrary.BreakVector` (`self.K2_GetActorLocation`)))
  (bind (_returnvalue_x_3 _returnvalue_y_3 _returnvalue_z_3) (`KismetMathLibrary.BreakVector` (`self.K2_GetActorLocation`)))
  (bind (_returnvalue_x_4 _returnvalue_y_4 _returnvalue_z_4) (`KismetMathLibrary.BreakVector` (`self.K2_GetActorLocation`)))
  (`SceneComponent.K2_SetWorldLocation` (`self.MovePosition1`) (`KismetMathLibrary.MakeVector` (`KismetMathLibrary.RandomFloatInRange` -2000.0 2000.0) (`KismetMathLibrary.RandomFloatInRange` -2000.0 2000.0) _returnvalue_z_4) false false)
  (`SceneComponent.K2_SetWorldLocation` (`self.MovePosition2`) (`KismetMathLibrary.MakeVector` (`KismetMathLibrary.RandomFloatInRange` -2000.0 2000.0) (`KismetMathLibrary.RandomFloatInRange` -2000.0 2000.0) _returnvalue_z) false false)
  (`SceneComponent.K2_SetWorldLocation` (`self.MovePosition3`) (`KismetMathLibrary.MakeVector` (`KismetMathLibrary.RandomFloatInRange` -2000.0 2000.0) (`KismetMathLibrary.RandomFloatInRange` -2000.0 2000.0) _returnvalue_z_2) false false)
  (`SceneComponent.K2_SetWorldLocation` (`self.MovePosition4`) (`KismetMathLibrary.MakeVector` (`KismetMathLibrary.RandomFloatInRange` -2000.0 2000.0) (`KismetMathLibrary.RandomFloatInRange` -2000.0 2000.0) _returnvalue_z_3) false false))

(fn `UserConstructionScript`)