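; Drone that harvests life force for the player by destroying stunned enemies.
; A Delay on Tick spaces out sweeps over all Enemy actors, regardless of distance, adding one LifeForce per stunned enemy and printing a debug message.
; BeginPlay caches the player and four patrol positions, then picks a random point.
; The timeline meant to lerp the drone between random points is never started, so patrol movement does not run.
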(event `self.ReceiveBeginPlay`
  (bind _asplayer (cast `/Game/Blueprints/Player` (`GameplayStatics.GetPlayerCharacter` 0)))
  (set `self.Player` _asplayer)
  (set `self.PatrolPoints` (`|MakeArray` (`SceneComponent.K2_GetComponentLocation` (`self.MovePosition1`)) (`SceneComponent.K2_GetComponentLocation` (`self.MovePosition2`)) (`SceneComponent.K2_GetComponentLocation` (`self.MovePosition3`)) (`SceneComponent.K2_GetComponentLocation` (`self.MovePosition4`))))
  (`self.GetRandomLocation`))

(event `self.ReceiveTick`
  (params (DeltaSeconds :type "Float (single-precision)"))
  (`KismetSystemLibrary.Delay` (`self.TimeBetweenCollecting`))
  (bind _outactors (`GameplayStatics.GetAllActorsOfClass` "/Game/Blueprints/Enemy.Enemy_C"))
  (for _array_element _outactors
    (if (`/Game/Blueprints/Enemy.isStunned` _array_element)
      (`self.K2_DestroyActor` _array_element)
      (`/Engine/EditorBlueprintResources/StandardMacros.IncrementInt` (`/Game/Blueprints/Player.LifeForce` (`self.Player`)))))
  (`KismetSystemLibrary.PrintString` "Collected"))

(fn `GetRandomLocation`
  (set `self.CurrentPatrolPoint` (`KismetMathLibrary.RandomIntegerInRange` 0 (- (`KismetArrayLibrary.Array_Length` (`self.PatrolPoints`)) 1))))

(fn `UserConstructionScript`)