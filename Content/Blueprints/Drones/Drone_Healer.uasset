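; Healer drone Blueprint that periodically restores the player's health, regardless of distance.
; BeginPlay caches the player and four patrol positions, then picks a random one.
; A Delay on Tick paces healing, adding a fixed amount while health is below a hardcoded threshold and printing a debug message.
; Timeline logic for lerping between random patrol points exists but is never triggered, so this graph never moves the drone.
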(event `self.ReceiveBeginPlay`
  (bind _asplayer (cast `/Game/Blueprints/Player` (`GameplayStatics.GetPlayerCharacter` 0)))
  (set `self.Player` _asplayer)
  (set `self.PatrolPoints` (`|MakeArray` (`SceneComponent.K2_GetComponentLocation` (`self.MovePosition1`)) (`SceneComponent.K2_GetComponentLocation` (`self.MovePosition2`)) (`SceneComponent.K2_GetComponentLocation` (`self.MovePosition3`)) (`SceneComponent.K2_GetComponentLocation` (`self.MovePosition4`))))
  (`self.GetRandomLocation`))

(event `self.ReceiveTick`
  (params (DeltaSeconds :type "Float (single-precision)"))
  (bind _player (`self.Player`))
  (bind _health (`/Game/Blueprints/Player.Health` _player))
  (`KismetSystemLibrary.Delay` (`self.TimeBetweenHealing`))
  (if (not (>= _health 1000))
    (set `/Game/Blueprints/Player.Health` (+ _health 100) _player)
    (`KismetSystemLibrary.PrintString` "Healed")))

(fn `GetRandomLocation`
  (set `self.CurrentPatrolPoint` (`KismetMathLibrary.RandomIntegerInRange` 0 (- (`KismetArrayLibrary.Array_Length` (`self.PatrolPoints`)) 1))))

(fn `UserConstructionScript`)