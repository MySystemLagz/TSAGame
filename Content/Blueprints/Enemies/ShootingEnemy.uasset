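; Ranged enemy actor that chases the player, shoots projectiles at them and drops skill points when killed.
; An AI MoveTo loop approaches to within a set range, snaps rotation toward the player, spawns an EnemyProjectile at a spawn component, then waits before repeating; failed moves retry after a shorter delay.
; Any damage reduces Health, and at zero it spawns PointsToDrop SkillPoint actors before destroying itself.
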(event `self.ReceiveBeginPlay`
  (bind _asplayer (cast `/Game/Blueprints/Player` (`GameplayStatics.GetPlayerCharacter` 0)))
  (bind _output_get (set `self.Player` _asplayer))
  (`|AIMoveTo` self (0.0 0.0 0.0) _output_get 1000.0 true :!label _label
    (:`OnSuccess`
      (`self.K2_SetActorRotation` (`KismetMathLibrary.FindLookAtRotation` (`self.K2_GetActorLocation`) (`self.K2_GetActorLocation` (`self.Player`))))
      (`|SpawnActorFromClass` "/Game/Blueprints/Enemies/EnemyProjectile.EnemyProjectile_C" (`SceneComponent.K2_GetComponentToWorld` (`self.ProjectileSpawnLocation`)) "Undefined" "OverrideRootScale" null null)
      (`KismetSystemLibrary.Delay` 1.0))
    (:`OnFail`
      _))
  (`KismetSystemLibrary.Delay` 1.0)
  (goto _label))

(event `self.ReceiveAnyDamage`
  (params (Damage :type "Float (single-precision)") (DamageType :type "DamageType Object Reference") (InstigatedBy :type "Controller Object Reference") (DamageCauser :type "Actor Object Reference"))
  (set `self.Health` (- (`self.Health`) Damage))
  (if (<= (`self.Health`) 0.0)
    (for _ (range 1 (+ (`self.PointsToDrop`) 1))
      (`|SpawnActorFromClass` "/Game/Blueprints/SkillPoint.SkillPoint_C" (`SceneComponent.K2_GetComponentToWorld` (`self.SkillPointSpawnLocation`)) "Undefined" "OverrideRootScale" null null))
    (`self.K2_DestroyActor`)))

(fn `UserConstructionScript`)