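; Bomber enemy Blueprint that chases the player and drops a grenade on arrival, sacrificing itself.
; On BeginPlay it tints its cube bright green and issues AIMoveTo toward the player character, retrying after a short delay whenever the move fails.
; When the move succeeds, it spawns an ImpuseGrenade at SkillPointSpawnLocation, adjusted for collisions but always spawned, then destroys itself.
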(event `self.ReceiveBeginPlay`
  (`MeshComponent.SetVectorParameterValueOnMaterials` (`self.Cube`) "BaseColor" (0.08 1.0 0.07))
  (`|AIMoveTo` self (0.0 0.0 0.0) (`GameplayStatics.GetPlayerCharacter` 0) :!label _label
    (:`OnSuccess`
      (`|SpawnActorFromClass` "/Game/Blueprints/Enemies/ImpuseGrenade.ImpuseGrenade_C" (`SceneComponent.K2_GetComponentToWorld` (`self.SkillPointSpawnLocation`)) "AdjustIfPossibleButAlwaysSpawn" "OverrideRootScale" null null)
      (`self.K2_DestroyActor`))
    (:`OnFail`
      (`KismetSystemLibrary.Delay` 1.0)
      (goto _label))))

(fn `UserConstructionScript`
  (`parent.UserConstructionScript`))