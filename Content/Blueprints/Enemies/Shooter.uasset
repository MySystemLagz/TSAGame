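; Shooter is a stationary enemy that fires projectiles at the player character, with its cube tinted red-orange on BeginPlay.
; A Delay-driven loop, with no Tick, snaps the actor to face the player and spawns an EnemyProjectile at ProjectileSpawnLocation.
; It repeats at random intervals of a few seconds and ends once the player character is invalid.
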(event `self.ReceiveBeginPlay`
  (bind _returnvalue (`GameplayStatics.GetPlayerCharacter` 0))
  (`MeshComponent.SetVectorParameterValueOnMaterials` (`self.Cube`) "BaseColor" (1.0 0.1 0.0))
  (`/Engine/EditorBlueprintResources/StandardMacros.IsValid` _returnvalue :!label _label
    (:`Is Valid`
      (`self.K2_SetActorRotation` (`KismetMathLibrary.FindLookAtRotation` (`self.K2_GetActorLocation`) (`self.K2_GetActorLocation` _returnvalue)))
      (`|SpawnActorFromClass` "/Game/Blueprints/Enemies/EnemyProjectile.EnemyProjectile_C" (`SceneComponent.K2_GetComponentToWorld` (`self.ProjectileSpawnLocation`)) "Undefined" "OverrideRootScale" null null)
      (`KismetSystemLibrary.Delay` (`KismetMathLibrary.RandomFloatInRange` 1.0 3.0))
      (goto _label))))

(fn `UserConstructionScript`)