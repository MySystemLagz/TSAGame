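; PlayerProjectile is a player projectile that knocks back Enemy characters it overlaps.
; A short delay after BeginPlay sets the Hit flag, so earlier overlaps are ignored.
; Each later overlap with an Enemy launches it away from the projectile, scaling horizontal push by Force and upward lift by Height, added to its existing velocity.
; The graph applies no damage and does not destroy the projectile.
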(event `self.ReceiveBeginPlay`
  (`KismetSystemLibrary.Delay` 0.2)
  (set `self.Hit` true))

(event `self.ReceiveActorBeginOverlap`
  (params (OtherActor :type "Actor Object Reference"))
  (if (`self.Hit`)
    (bind _asenemy (cast `/Game/Blueprints/Enemy` OtherActor))
    (bind (_returnvalue_x _returnvalue_y) (`KismetMathLibrary.BreakVector` (* (`KismetMathLibrary.GetDirectionUnitVector` (`self.K2_GetActorLocation`) (`self.K2_GetActorLocation` _asenemy)) (`self.Force`))))
    (bind (_returnvalue_x_2 _returnvalue_y_2 _returnvalue_z) (`KismetMathLibrary.BreakVector` (`self.GetActorUpVector` _asenemy)))
    (`Character.LaunchCharacter` _asenemy (`KismetMathLibrary.MakeVector` _returnvalue_x _returnvalue_y (* (`self.Height`) _returnvalue_z)) false false)))

(fn `UserConstructionScript`)