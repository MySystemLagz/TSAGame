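; KillZ is a kill volume that removes enemies, the player and player projectiles that enter its box.
; On box overlap, it destroys any actor tagged Enemy, then uses casts to identify a Player or PlayerProjectile and destroy it.
; A player death also restarts play by opening the Game level after a retry delay.
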(event `self.Box.OnComponentBeginOverlap`
  (params (OverlappedComponent :type "PrimitiveComponent Object Reference") (OtherActor :type "Actor Object Reference") (OtherComp :type "PrimitiveComponent Object Reference") (OtherBodyIndex :type Integer) (bFromSweep :type Boolean) (SweepResult :type "HitResult Structure (by ref)"))
  (for _array_element (`Actor.Tags` OtherActor)
    (if (== _array_element "Enemy")
      (`self.K2_DestroyActor` OtherActor)))
  (bind _asplayer (cast `/Game/Blueprints/Player` OtherActor)
    (:`then`
      (`self.K2_DestroyActor` _asplayer)
      (`KismetSystemLibrary.Delay` (`self.RetryLevelDelay`))
      (`GameplayStatics.OpenLevel` "Game"))
    (:`CastFailed`
      (bind _asplayer_projectile (cast `/Game/Blueprints/PlayerProjectile` OtherActor))
      (`self.K2_DestroyActor` _asplayer_projectile))))

(fn `UserConstructionScript`)