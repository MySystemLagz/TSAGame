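; Enemy actor that chases the player, hurts them on contact and drops skill points when killed.
; BeginPlay starts an endless AIMoveTo loop toward the player, retrying one second after each success or failure.
; Overlapping the Cube deals Damage through the player's TakeDamage.
; Its own TakeDamage reduces Health, then at zero spawns PointsToDrop SkillPoint pickups at a spawn component before destroying itself.
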(event `self.ReceiveBeginPlay`
  (bind _asplayer (cast `/Game/Blueprints/Player` (`GameplayStatics.GetPlayerCharacter` 0)))
  (bind _output_get (set `self.Player` _asplayer))
  (`|AIMoveTo` self (0.0 0.0 0.0) _output_get 5.0 true :!label _label
    (:`OnSuccess`
      _)
    (:`OnFail`
      _))
  (`KismetSystemLibrary.Delay` 1.0)
  (goto _label))

(event `TakeDamage`
  (params (DamageAmount :type "Float (double-precision)"))
  ;[1 1 1] Take Damage Event
  (set `self.Health` (- (`self.Health`) DamageAmount))
  (if (<= (`self.Health`) 0.0)
    (for _ (range 1 (+ (`self.PointsToDrop`) 1))
      (`|SpawnActorFromClass` "/Game/Blueprints/SkillPoint.SkillPoint_C" (`SceneComponent.K2_GetComponentToWorld` (`self.SkillPointSpawnLocation`)) "AdjustIfPossibleButAlwaysSpawn" "OverrideRootScale" null null))
    (`self.K2_DestroyActor`)))

(event `self.Cube.OnComponentBeginOverlap`
  (params (OverlappedComponent :type "PrimitiveComponent Object Reference") (OtherActor :type "Actor Object Reference") (OtherComp :type "PrimitiveComponent Object Reference") (OtherBodyIndex :type Integer) (bFromSweep :type Boolean) (SweepResult :type "HitResult Structure (by ref)"))
  (bind _asplayer (cast `/Game/Blueprints/Player` OtherActor))
  (`/Game/Blueprints/Player.Take Damage` _asplayer (`self.Damage`)))

(fn `UserConstructionScript`)